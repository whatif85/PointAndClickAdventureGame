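; BP_Hotspot is a base interactive hotspot for a point-and-click adventure, with default responses to verbs like Look at, Use, Open and Pick up.
; Cursor enter and exit on its static mesh notify BP_AdventureController of the hovered hotspot.
; Each verb event only prints a refusal line.
; The construction script moves the WalkToPoint component to the WalkToPosition world location.
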(event `self.StaticMeshComponent.OnBeginCursorOver`
  (params (TouchedComponent :type "PrimitiveComponent Object Reference"))
  (bind _asbp_adventure_controller (cast `/Game/PointAndClick/Blueprints/BP_AdventureController` (`GameplayStatics.GetPlayerController` 0)))
  (`/Game/PointAndClick/Blueprints/BP_AdventureController.MouseEnterHotspot` _asbp_adventure_controller self))

(event `self.StaticMeshComponent.OnEndCursorOver`
  (params (TouchedComponent :type "PrimitiveComponent Object Reference"))
  (bind _asbp_adventure_controller (cast `/Game/PointAndClick/Blueprints/BP_AdventureController` (`GameplayStatics.GetPlayerController` 0)))
  (`/Game/PointAndClick/Blueprints/BP_AdventureController.MouseExitHotspot` _asbp_adventure_controller))

(event `/Game/PointAndClick/Blueprints/BPI_VerbInteraction.OnPull`
  (`KismetSystemLibrary.PrintString` "I can't move it."))

(event `/Game/PointAndClick/Blueprints/BPI_VerbInteraction.OnPush`
  (`KismetSystemLibrary.PrintString` "I can't move it."))

(event `/Game/PointAndClick/Blueprints/BPI_VerbInteraction.OnUse`
  (`KismetSystemLibrary.PrintString` "That doesn't seem to work."))

(event `/Game/PointAndClick/Blueprints/BPI_VerbInteraction.OnTalkTo`
  (`KismetSystemLibrary.PrintString` "Hmmm... Maybe not."))

(event `/Game/PointAndClick/Blueprints/BPI_VerbInteraction.OnLookAt`
  (`KismetSystemLibrary.PrintString` "I don't see anything special about it."))

(event `/Game/PointAndClick/Blueprints/BPI_VerbInteraction.OnClose`
  (`KismetSystemLibrary.PrintString` "I can't close that."))

(event `/Game/PointAndClick/Blueprints/BPI_VerbInteraction.OnOpen`
  (`KismetSystemLibrary.PrintString` "I can't open that."))

(event `/Game/PointAndClick/Blueprints/BPI_VerbInteraction.OnGive`
  (`KismetSystemLibrary.PrintString` "I can't give that."))

(event `/Game/PointAndClick/Blueprints/BPI_VerbInteraction.OnPickup`
  (`KismetSystemLibrary.PrintString` "I can't pick that up."))

(fn `UserConstructionScript`
  (`SceneComponent.K2_SetWorldLocation` (`self.WalkToPoint`) (`self.WalkToPosition`) false false))