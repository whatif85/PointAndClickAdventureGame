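; Blueprint function library for a point-and-click adventure game, giving global shortcuts to core gameplay objects and common actions.
; Getters cast to the adventure game instance, player controller and its character, and find the HUD through a widget class search.
; Helpers build on these to trigger room loading via the game instance, lock or unlock player input, assign the room camera, and toggle a black screen.
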(fn `ActivateCurrentCamera`
  (`/Game/PointAndClick/Blueprints/Characters/BP_AdventureCharacter.AssignRoomCamera` (`self.GetAdventureCharacter` null)))

(fn `GetAdventureCharacter`
  (returns (AdventureCharacter :type "/Game/PointAndClick/Blueprints/Characters/BP_AdventureCharacter Object Reference"))
  (bind _asbp_adventure_controller (cast `/Game/PointAndClick/Blueprints/BP_AdventureController` (`GameplayStatics.GetPlayerController` null)))
  (return (`/Game/PointAndClick/Blueprints/BP_AdventureController.PlayerCharacter` _asbp_adventure_controller)))

(fn `GetAdventureController`
  (returns (AdventureController :type "/Game/PointAndClick/Blueprints/BP_AdventureController Object Reference"))
  (bind _asbp_adventure_controller (cast `/Game/PointAndClick/Blueprints/BP_AdventureController` (`GameplayStatics.GetPlayerController` null)))
  (return _asbp_adventure_controller))

(fn `GetAdventureInstance`
  (returns (AdventureInstance :type "/Game/PointAndClick/Blueprints/BP_AdventureInstance Object Reference"))
  (bind _asbp_adventure_instance (cast `/Game/PointAndClick/Blueprints/BP_AdventureInstance` (`GameplayStatics.GetGameInstance` null)))
  (return _asbp_adventure_instance))

(fn `GetHUD`
  (returns (Output :type "/Game/PointAndClick/Blueprints/Widgets/WBP_HUD Object Reference"))
  (bind _foundwidgets (`WidgetBlueprintLibrary.GetAllWidgetsOfClass` null "/Game/PointAndClick/Blueprints/Widgets/WBP_HUD.WBP_HUD_C"))
  (return (`|GetArrayItem` _foundwidgets)))

(fn `HideBlackScreen`
  (`Widget.SetVisibility` (`/Game/PointAndClick/Blueprints/Widgets/WBP_HUD.BlackScreen` (`self.GetHUD` null)) "Hidden"))

(fn `LoadRoom`
  (params (DoorLoad :type "/Game/PointAndClick/Blueprints/Hotspots/BP_Hotspot_Door Object Reference"))
  (bind _adventureinstance (`self.GetAdventureInstance` null))
  (set `/Game/PointAndClick/Blueprints/BP_AdventureInstance.CurrentDoor` DoorLoad _adventureinstance)
  (`/Game/PointAndClick/Blueprints/BP_AdventureInstance.EventLoadRoom` _adventureinstance))

(fn `LoadStartingRoom`
  (`/Game/PointAndClick/Blueprints/BP_AdventureInstance.EventLoadStartingRoom` (`self.GetAdventureInstance` null)))

(fn `LockPlayerInput`
  (set `/Game/PointAndClick/Blueprints/BP_AdventureController.bLockInput` true (`self.GetAdventureController` null)))

(fn `ShowBlackScreen`
  (`Widget.SetVisibility` (`/Game/PointAndClick/Blueprints/Widgets/WBP_HUD.BlackScreen` (`self.GetHUD` null)) "Visible"))

(fn `UnlockPlayerInput`
  (set `/Game/PointAndClick/Blueprints/BP_AdventureController.bLockInput` false (`self.GetAdventureController` null)))