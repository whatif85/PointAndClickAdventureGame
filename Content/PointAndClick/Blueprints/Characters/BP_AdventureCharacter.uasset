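; Player character for a point-and-click adventure, a pixel-art flipbook sprite that walks, idles, plays actions and speaks barks.
; Tick turns velocity into side, up or down walk animations, mirroring the sprite by scale, then a DoOnce picks the matching idle and snaps position to whole units on stopping.
; Timed widget barks and one-shot animations, which restore the prior state, advance the adventure controller's task index when finished.
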(event `self.ReceiveBeginPlay`
  (bind _aswbp_bark_text (cast `/Game/PointAndClick/Blueprints/Widgets/WBP_BarkText` (`WidgetComponent.GetUserWidgetObject` (`self.BarkWidget`))))
  (`/Game/PointAndClick/Blueprints/Widgets/WBP_BarkText.SetBarkText` _aswbp_bark_text ""))

(event `self.ReceiveTick`
  (params (DeltaSeconds :type "Float (single-precision)"))
  (`self.IsCharacterMoving?`
    (:`Yes`
      (`self.SetSpeed`
        (:`Out`
          (`self.GetPrimaryDirection`
            (:`Horizontal`
              (`self.SetHorizontalAnimation`
                (:`Out`
                  (goto _label :!via `Reset`))))
            (:`Vertical`
              (`self.SetVerticalAnimation`
                (:`Out`
                  (goto _label :!via `Reset`))))))))
    (:`No`
      (`/Engine/EditorBlueprintResources/StandardMacros.DoOnce` false :!label _label
        (:`Completed`
          (`self.DetermineIdleDirection`
            (:`Out`
              (`self.SetPosition`))))))))

(event `ResetIdle`
  (goto _label :!via `Reset`))

(event `BarkDelay`
  (`Timeline|BarkTimeline` :!via `PlayFromStart` :!label _label_2
    (:`Finished`
      (`self.ClearBark`)
      (`/Game/PointAndClick/Blueprints/BP_AdventureController.IncrementTaskIndex` (`/Game/PointAndClick/Blueprints/BFL_AdventureLibrary.GetAdventureController`)))))

(event `BarkReset`
  (goto _label_2 :!via `Stop`))

(event `PlayAnimation`
  (params (Animation :type "/Game/PointAndClick/Blueprints/Enums/ENUM_CurrentAnimState Enum" :default "NewEnumerator0"))
  (`self.PlayAnimationSequence` Animation
    (:`Out`
      (`/Game/PointAndClick/Blueprints/BP_AdventureController.IncrementTaskIndex` (`/Game/PointAndClick/Blueprints/BFL_AdventureLibrary.GetAdventureController`)))))

(fn `ClearBark`
  (set `self.bBarking` false)
  (bind _aswbp_bark_text (cast `/Game/PointAndClick/Blueprints/Widgets/WBP_BarkText` (`WidgetComponent.GetUserWidgetObject` (`self.BarkWidget`))))
  (`/Game/PointAndClick/Blueprints/Widgets/WBP_BarkText.SetBarkText` _aswbp_bark_text "")
  (`self.BarkReset`))

(fn `PlayerBark`
  (params (BarkText :type String))
  (if (`self.bBarking`)
    (`self.ClearBark`))
  (set `self.bBarking` true)
  (bind _aswbp_bark_text (cast `/Game/PointAndClick/Blueprints/Widgets/WBP_BarkText` (`WidgetComponent.GetUserWidgetObject` (`self.BarkWidget`))))
  (`/Game/PointAndClick/Blueprints/Widgets/WBP_BarkText.SetBarkText` _aswbp_bark_text BarkText)
  (`self.BarkDelay`))

(fn `SetFacingDirection`
  (params (FacingDirection :type "/Game/PointAndClick/Blueprints/Enums/ENUM_FacingDirection Enum" :default "NewEnumerator0"))
  (bind _sprite (`self.Sprite`))
  (switch `/Game/PointAndClick/Blueprints/Enums/ENUM_FacingDirection` FacingDirection
    (:`NewEnumerator0`
      (`self.SetAnimationState` "NewEnumerator2"
        (:`Out`
          _)))
    (:`NewEnumerator1`
      (`SceneComponent.SetRelativeScale3D` _sprite (-0.25 0.25 0.25))
      (`self.SetAnimationState` "NewEnumerator0" :!label _label
        (:`Out`
          _)))
    (:`NewEnumerator2`
      (`self.SetAnimationState` "NewEnumerator1"
        (:`Out`
          _)))
    (:`NewEnumerator3`
      (`SceneComponent.SetRelativeScale3D` _sprite (0.25 0.25 0.25))
      (goto _label)))
  (return))

(fn `SetPosition`
  (bind _capsulecomponent (`self.CapsuleComponent`))
  (bind (_returnvalue_x _returnvalue_y _returnvalue_z) (`KismetMathLibrary.BreakVector` (`SceneComponent.K2_GetComponentLocation` _capsulecomponent)))
  (`SceneComponent.K2_SetWorldLocation` _capsulecomponent (`KismetMathLibrary.MakeVector` (`KismetMathLibrary.Conv_IntToDouble` (`KismetMathLibrary.FFloor` _returnvalue_x)) (`KismetMathLibrary.Conv_IntToDouble` (`KismetMathLibrary.FFloor` _returnvalue_y)) _returnvalue_z) false false))

(fn `TeleportToLocation`
  (params (Location :type "Vector Structure"))
  (`SceneComponent.K2_SetWorldLocation` (`self.CapsuleComponent`) Location false false))

(fn `UserConstructionScript`)