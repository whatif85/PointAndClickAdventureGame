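; Adventure instance for a point-and-click game that handles loading the starting room and moving between rooms through doors.
; Rooms are streamed levels swapped behind a black screen, with player input locked during door transitions.
; After each load, FindDoor searches door hotspots for a matching label and places the character at its walk-to position and facing.
; Transitions end by interrupting the controller's current action.
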(event `EventLoadStartingRoom`
  (`/Game/PointAndClick/Blueprints/BFL_AdventureLibrary.ShowBlackScreen`)
  (`GameplayStatics.LoadStreamLevel` (`self.StartingLevel`) true true)
  (`self.FindDoor` (`self.StartingDoorLabel`))
  (`KismetSystemLibrary.Delay` 0.25)
  (`/Game/PointAndClick/Blueprints/BFL_AdventureLibrary.HideBlackScreen`)
  (`/Game/PointAndClick/Blueprints/BP_AdventureController.InterruptAction` (`/Game/PointAndClick/Blueprints/BFL_AdventureLibrary.GetAdventureController`)))

(event `EventLoadRoom`
  (bind _currentdoor (`self.CurrentDoor`))
  (`/Game/PointAndClick/Blueprints/BFL_AdventureLibrary.LockPlayerInput`)
  (`/Game/PointAndClick/Blueprints/BFL_AdventureLibrary.ShowBlackScreen`)
  (`GameplayStatics.LoadStreamLevel` (`/Game/PointAndClick/Blueprints/Hotspots/BP_Hotspot_Door.LevelToLoad` _currentdoor) true true)
  (set `self.TempDoorLabel` (`/Game/PointAndClick/Blueprints/Hotspots/BP_Hotspot_Door.DoorLabel` _currentdoor))
  (`GameplayStatics.UnloadStreamLevel` (`/Game/PointAndClick/Blueprints/Hotspots/BP_Hotspot_Door.CurrentLevel` _currentdoor))
  (`self.FindDoor` (`self.TempDoorLabel`))
  (`KismetSystemLibrary.Delay` 0.5)
  (`/Game/PointAndClick/Blueprints/BFL_AdventureLibrary.HideBlackScreen`)
  (`/Game/PointAndClick/Blueprints/BP_AdventureController.InterruptAction` (`/Game/PointAndClick/Blueprints/BFL_AdventureLibrary.GetAdventureController`))
  (`/Game/PointAndClick/Blueprints/Characters/BP_AdventureCharacter.ClearBark` (`/Game/PointAndClick/Blueprints/BFL_AdventureLibrary.GetAdventureCharacter`))
  (`/Game/PointAndClick/Blueprints/BFL_AdventureLibrary.UnlockPlayerInput`))

(fn `FindDoor`
  (params (DoorLabel :type String))
  (bind _adventurecharacter (`/Game/PointAndClick/Blueprints/BFL_AdventureLibrary.GetAdventureCharacter`))
  (bind _outactors (`GameplayStatics.GetAllActorsOfClass` "/Game/PointAndClick/Blueprints/Hotspots/BP_Hotspot_Door.BP_Hotspot_Door_C"))
  (for _array_element _outactors
    (if (== (`/Game/PointAndClick/Blueprints/Hotspots/BP_Hotspot_Door.DoorLabel` _array_element) DoorLabel)
      (`/Game/PointAndClick/Blueprints/Characters/BP_AdventureCharacter.TeleportToLocation` _adventurecharacter (`/Game/PointAndClick/Blueprints/Hotspots/BP_Hotspot.WalkToPosition` _array_element))
      (`/Game/PointAndClick/Blueprints/Characters/BP_AdventureCharacter.SetFacingDirection` _adventurecharacter (`/Game/PointAndClick/Blueprints/Hotspots/BP_Hotspot.FacingDirection` _array_element))
      (return)))
  (`KismetSystemLibrary.PrintString` "Hello")
  (return))