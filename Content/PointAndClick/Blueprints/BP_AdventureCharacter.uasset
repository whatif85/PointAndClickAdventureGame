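; Point-and-click adventure player character that plays directional pixel-art flipbook animations.
; On BeginPlay it takes the overlapping BP_AdventureCamera as view target and registers itself as that camera's player.
; Each tick, local velocity's dominant axis picks the walk flipbook, mirroring the side sprite for left, and the last direction picks the idle one.
; A DoOnce floors X/Y location on stopping to keep pixels aligned; SetFacingDirection sets idle facing directly.
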(event `self.ReceiveBeginPlay`
  (`KismetSystemLibrary.Delay` 0.0)
  (bind _asbp_adventure_camera (cast `/Game/PointAndClick/Blueprints/BP_AdventureCamera` (`|GetArrayItem` (`PrimitiveComponent.GetOverlappingActors` (`self.CapsuleComponent`) "/Game/PointAndClick/Blueprints/BP_AdventureCamera.BP_AdventureCamera_C"))))
  (`PlayerController.SetViewTargetWithBlend` (`GameplayStatics.GetPlayerController` 0) _asbp_adventure_camera 0.0 "VTBlend_Linear" 0.0 false)
  (set `/Game/PointAndClick/Blueprints/BP_AdventureCamera.Player` self _asbp_adventure_camera))

(event `self.ReceiveTick`
  (params (DeltaSeconds :type "Float (single-precision)"))
  (`self.IsCharacterMoving?`
    (:`Yes`
      (`self.SetSpeed`
        (:`Out`
          (`self.GetPrimaryDirection`
            (:`Horizontal`
              (`self.SetHorizontalAnimation`
                (:`Out`
                  (goto _label :!via `Reset`))))
            (:`Vertical`
              (`self.SetVerticalAnimation`
                (:`Out`
                  (goto _label :!via `Reset`))))))))
    (:`No`
      (`self.DetermineIdleDirection`
        (:`Out`
          (`/Engine/EditorBlueprintResources/StandardMacros.DoOnce` false :!label _label
            (:`Completed`
              (`self.SetPosition`))))))))

(fn `SetFacingDirection`
  (params (FacingDirection :type "/Game/PointAndClick/Blueprints/Enums/ENUM_FacingDirection Enum" :default "NewEnumerator0"))
  (bind _sprite (`self.Sprite`))
  (switch `/Game/PointAndClick/Blueprints/Enums/ENUM_FacingDirection` FacingDirection
    (:`NewEnumerator0`
      (`self.SetAnimationState` "NewEnumerator2"
        (:`Out`
          _)))
    (:`NewEnumerator1`
      (`SceneComponent.SetRelativeScale3D` _sprite (1.0 1.0 1.0))
      (`self.SetAnimationState` "NewEnumerator0" :!label _label
        (:`Out`
          _)))
    (:`NewEnumerator2`
      (`self.SetAnimationState` "NewEnumerator1"
        (:`Out`
          _)))
    (:`NewEnumerator3`
      (`SceneComponent.SetRelativeScale3D` _sprite (-1.0 1.0 1.0))
      (goto _label)))
  (return))

(fn `SetPosition`
  (bind _capsulecomponent (`self.CapsuleComponent`))
  (bind (_returnvalue_x _returnvalue_y _returnvalue_z) (`KismetMathLibrary.BreakVector` (`SceneComponent.K2_GetComponentLocation` _capsulecomponent)))
  (`SceneComponent.K2_SetWorldLocation` _capsulecomponent (`KismetMathLibrary.MakeVector` (`KismetMathLibrary.Conv_IntToDouble` (`KismetMathLibrary.FFloor` _returnvalue_x)) (`KismetMathLibrary.Conv_IntToDouble` (`KismetMathLibrary.FFloor` _returnvalue_y)) _returnvalue_z) false false))

(fn `UserConstructionScript`)