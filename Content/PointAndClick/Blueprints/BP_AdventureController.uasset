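; Player controller for a verb-based point-and-click adventure, handling clicks, hover targets and interaction text.
; Clicks AI-move the character to a location or a hotspot's walk-to point, then dispatch the active verb to that hotspot.
; Multi-step task interactions block clicks and re-fire the verb as TaskIndex increments, with events for barks, facing, waits and animations.
; Inventory clicks route verbs to items, with Give and Use still debug stubs.
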(event `self.ReceiveBeginPlay`
  (`self.UpdateInteractionText`)
  (`/Game/PointAndClick/Blueprints/BFL_AdventureLibrary.LoadStartingRoom`))

(event `Key|LeftMouseButton`
  (params (Key :type "Key Structure"))
  (:`Pressed`
    (`self.GetClicked`
      (:`Hotspot`
        (`self.WalkToHotspot`
          (:`Out`
            (`self.PerformInteraction`))))
      (:`Nothing`
        (`self.WalkToLocation`)))))

(event `ItemClicked`
  (`self.PerformItemInteraction`))

(event `TaskBark`
  (params (BarkText :type String))
  (`/Game/PointAndClick/Blueprints/Characters/BP_AdventureCharacter.PlayerBark` (`self.PlayerCharacter`) BarkText))

(event `TaskFaceDirection`
  (params (FacingDirection :type "/Game/PointAndClick/Blueprints/Enums/ENUM_FacingDirection Enum" :default "NewEnumerator0"))
  (`/Game/PointAndClick/Blueprints/Characters/BP_AdventureCharacter.SetFacingDirection` (`self.PlayerCharacter`) FacingDirection)
  (`KismetSystemLibrary.Delay` 0.2)
  (`self.IncrementTaskIndex`))

(event `TaskWait`
  (params (WaitTime :type "Float (double-precision)"))
  (`KismetSystemLibrary.Delay` WaitTime)
  (`self.IncrementTaskIndex`))

(event `TaskPlayAnimation`
  (params (Animation :type "/Game/PointAndClick/Blueprints/Enums/ENUM_CurrentAnimState Enum" :default "NewEnumerator0"))
  (`/Game/PointAndClick/Blueprints/Characters/BP_AdventureCharacter.PlayAnimation` (`self.PlayerCharacter`) Animation))

(fn `AssignVerb`
  (params (Verb :type "/Game/PointAndClick/Blueprints/Enums/ENUM_VerbUsed Enum" :default "NewEnumerator0"))
  (set `self.ActiveVerb` Verb)
  (`self.UpdateInteractionText`))

(fn `BeginTaskInteraction`
  (set `self.bPerformingTaskInteraction` true)
  (`self.IncrementTaskIndex`))

(fn `EndTaskInteraction`
  (set `self.TaskIndex` 0)
  (set `self.bPerformingTaskInteraction` false)
  (`self.InterruptAction`))

(fn `IncrementTaskIndex`
  (if (`self.bPerformingTaskInteraction`)
    (`/Engine/EditorBlueprintResources/StandardMacros.IncrementInt` (`self.TaskIndex`)
      (:`  `
        (`self.PerformInteraction`)))))

(fn `InterruptAction`
  (`NavMovementComponent.StopActiveMovement` (`Character.CharacterMovement` (`self.PlayerCharacter`)))
  (set `self.ActiveVerb` "NewEnumerator0")
  (set `self.TargetHotspot` null)
  (set `self.bHotspotInteraction` false)
  (`/Game/PointAndClick/Blueprints/Characters/BP_AdventureCharacter.ResetIdle` (`self.PlayerCharacter`))
  (`self.InterruptingAction`))

(fn `MouseEnterHotspot`
  (params (Hotspot :type "/Game/PointAndClick/Blueprints/Hotspots/BP_Hotspot Object Reference"))
  (if (or (`self.bPerformingTaskInteraction`) (`self.bHotspotInteraction`))
    (set `self.NewHotspot` Hotspot)
    (else
      (set `self.TargetHotspot` Hotspot)
      (`self.UpdateInteractionText`))))

(fn `MouseEnterInventoryItem`
  (params (ItemSlot :type "/Game/PointAndClick/Blueprints/Widgets/WBP_ItemSlot Object Reference"))
  (if (not (or (`self.bHotspotInteraction`) (`self.bPerformingTaskInteraction`)))
    (set `self.TargetInventorySlot` ItemSlot)
    (`self.UpdateInteractionText`)))

(fn `MouseExitHotspot`
  (if (not (or (`self.bPerformingTaskInteraction`) (`self.bHotspotInteraction`)))
    (set `self.TargetHotspot` null))
  (set `self.NewHotspot` null)
  (`self.UpdateInteractionText`))

(fn `MouseExitInventoryItem`
  (if (not (or (`self.bHotspotInteraction`) (`self.bPerformingTaskInteraction`)))
    (set `self.TargetInventorySlot` null)
    (`self.UpdateInteractionText`)))

(fn `UserConstructionScript`)