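; Point-and-click hotspot for a poster, overriding the parent's Look At and Pick Up verb responses.
; Each verb runs as a step sequence switched on the PlayerController's TaskIndex: begin interaction, face the hotspot, then barks, turns or animation.
; The default case releases the player: Look At ends the task, while Pick Up interrupts it, barks about a pickle, clears the verb and only debug-prints the inventory add.
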(event `/Game/PointAndClick/Blueprints/Interfaces/BPI_VerbInteraction.OnLookAt`
  (switch `int` (`/Game/PointAndClick/Blueprints/BP_AdventureController.TaskIndex` (`self.PlayerController`))
    (:`Default`
      (`self.EndTaskInteraction`) ; Player is free to move only after the interaction is completed.
    )
    (:`0`
      (`self.BeginTaskInteraction`))
    (:`1`
      (`self.Face Hotspot`))
    (:`2`
      (`self.Bark` "Hmmm..."))
    (:`3`
      (`self.Bark` "There's something peculiar about this poster."))
    (:`4`
      (`self.FaceDirection` "NewEnumerator2"))
    (:`5`
      (`self.Bark` "Man, what a poster!"))))

(event `/Game/PointAndClick/Blueprints/Interfaces/BPI_VerbInteraction.OnPickup`
  (switch `int` (`/Game/PointAndClick/Blueprints/BP_AdventureController.TaskIndex` (`self.PlayerController`))
    (:`Default`
      (`self.InterruptTaskInteraction`) ; Allows free movement after playing pick up animation.
      (`KismetSystemLibrary.PrintString` "DEBUG: Added Pickle to Inventory")
      (`self.Bark` "There's a pickle behind this poster!")
      (`self.ClearVerb`))
    (:`0`
      (`self.BeginTaskInteraction`))
    (:`1`
      (`self.Face Hotspot`))
    (:`2`
      (`self.PlayAnimation` "NewEnumerator10"))))

(fn `UserConstructionScript`
  (`parent.UserConstructionScript`))