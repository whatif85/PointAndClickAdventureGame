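; BP_Hotspot is an interactable point-and-click adventure object that reports cursor hover to BP_AdventureController and provides default responses to verbs.
; Each verb event faces the target hotspot's direction, barks a refusal line (except Walk To), then interrupts the action.
; Helper functions forward barks, waits, animations, facing and inventory changes to the controller, mostly as tasks.
; The construction script moves WalkToPoint to the WalkToPosition variable.
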(event `self.ReceiveBeginPlay`
  (bind _asbp_adventure_controller (cast `/Game/PointAndClick/Blueprints/BP_AdventureController` (`GameplayStatics.GetPlayerController` 0)))
  (set `self.PlayerController` _asbp_adventure_controller))

(event `self.StaticMeshComponent.OnBeginCursorOver`
  (params (TouchedComponent :type "PrimitiveComponent Object Reference"))
  (`/Game/PointAndClick/Blueprints/BP_AdventureController.MouseEnterHotspot` (`self.PlayerController`) self))

(event `self.StaticMeshComponent.OnEndCursorOver`
  (params (TouchedComponent :type "PrimitiveComponent Object Reference"))
  (`/Game/PointAndClick/Blueprints/BP_AdventureController.MouseExitHotspot` (`self.PlayerController`)))

(event `/Game/PointAndClick/Blueprints/Interfaces/BPI_VerbInteraction.OnPull`
  (`self.Face Hotspot`)
  (`self.Bark` "I can't move it.")
  (`self.ClearVerb`))

(event `/Game/PointAndClick/Blueprints/Interfaces/BPI_VerbInteraction.OnPush`
  (`self.Face Hotspot`)
  (`self.Bark` "I can't move it.")
  (`self.ClearVerb`))

(event `/Game/PointAndClick/Blueprints/Interfaces/BPI_VerbInteraction.OnUse`
  (`self.Face Hotspot`)
  (`self.Bark` "That doesn't seem to work.")
  (`self.ClearVerb`))

(event `/Game/PointAndClick/Blueprints/Interfaces/BPI_VerbInteraction.OnTalkTo`
  (`self.Face Hotspot`)
  (`self.Bark` "Hmmm... Maybe not.")
  (`self.ClearVerb`))

(event `/Game/PointAndClick/Blueprints/Interfaces/BPI_VerbInteraction.OnLookAt`
  (`self.Face Hotspot`)
  (`self.Bark` "I don't see anything special about it.")
  (`self.ClearVerb`))

(event `/Game/PointAndClick/Blueprints/Interfaces/BPI_VerbInteraction.OnClose`
  (`self.Face Hotspot`)
  (`self.Bark` "That doesn't seem to close.")
  (`self.ClearVerb`))

(event `/Game/PointAndClick/Blueprints/Interfaces/BPI_VerbInteraction.OnOpen`
  (`self.Face Hotspot`)
  (`self.Bark` "That doesn't seem to open.")
  (`self.ClearVerb`))

(event `/Game/PointAndClick/Blueprints/Interfaces/BPI_VerbInteraction.OnGive`
  (`self.Face Hotspot`)
  (`self.Bark` "I can't give that.")
  (`self.ClearVerb`))

(event `/Game/PointAndClick/Blueprints/Interfaces/BPI_VerbInteraction.OnPickup`
  (`self.Face Hotspot`)
  (`self.Bark` "I can't pick that up.")
  (`self.ClearVerb`))

(event `/Game/PointAndClick/Blueprints/Interfaces/BPI_VerbInteraction.OnWalkTo`
  (`self.Face Hotspot`)
  (`self.ClearVerb`))

(fn `AddItemToInventory`
  (params (ItemToAdd :type "/Game/PointAndClick/Blueprints/Enums/ENUM_ItemList Enum" :default "NewEnumerator0"))
  (`/Game/PointAndClick/Blueprints/BP_AdventureController.TaskAddItemToInventory` (`/Game/PointAndClick/Blueprints/BFL_AdventureLibrary.GetAdventureController`) ItemToAdd))

(fn `Bark`
  (params (BarkText :type String))
  (`/Game/PointAndClick/Blueprints/BP_AdventureController.TaskBark` (`self.PlayerController`) BarkText))

(fn `BeginTaskInteraction`
  (`/Game/PointAndClick/Blueprints/BP_AdventureController.BeginTaskInteraction` (`self.PlayerController`)))

(fn `ClearVerb`
  (`/Game/PointAndClick/Blueprints/BP_AdventureController.InterruptAction` (`self.PlayerController`)))

(fn `EndTaskInteraction`
  (`/Game/PointAndClick/Blueprints/BP_AdventureController.EndTaskInteraction` (`self.PlayerController`)))

(fn `Face Hotspot`
  (bind _playercontroller (`self.PlayerController`))
  (bind _targethotspot (`/Game/PointAndClick/Blueprints/BP_AdventureController.TargetHotspot` _playercontroller))
  (`/Engine/EditorBlueprintResources/StandardMacros.IsValid` _targethotspot
    (:`Is Valid`
      (`/Game/PointAndClick/Blueprints/BP_AdventureController.TaskFaceDirection` _playercontroller (`/Game/PointAndClick/Blueprints/Hotspots/BP_Hotspot.FacingDirection` _targethotspot)))))

(fn `FaceDirection`
  (params (FacingDirection :type "/Game/PointAndClick/Blueprints/Enums/ENUM_FacingDirection Enum" :default "NewEnumerator0"))
  (`/Game/PointAndClick/Blueprints/BP_AdventureController.TaskFaceDirection` (`self.PlayerController`) FacingDirection))

(fn `InterruptTaskInteraction`
  (bind _playercontroller (`self.PlayerController`))
  (set `/Game/PointAndClick/Blueprints/BP_AdventureController.TaskIndex` 0 _playercontroller)
  (set `/Game/PointAndClick/Blueprints/BP_AdventureController.bPerformingTaskInteraction` false _playercontroller))

(fn `PlayAnimation`
  (params (Animation :type "/Game/PointAndClick/Blueprints/Enums/ENUM_CurrentAnimState Enum" :default "NewEnumerator0"))
  (`/Game/PointAndClick/Blueprints/BP_AdventureController.TaskPlayAnimation` (`self.PlayerController`) Animation))

(fn `RemoveItemFromInventory`
  (params (ItemToRemove :type "/Game/PointAndClick/Blueprints/Enums/ENUM_ItemList Enum" :default "NewEnumerator0"))
  (`/Game/PointAndClick/Blueprints/BP_AdventureController.RemoveItemFromInventory` (`/Game/PointAndClick/Blueprints/BFL_AdventureLibrary.GetAdventureController`) ItemToRemove))

(fn `UserConstructionScript`
  (`SceneComponent.K2_SetWorldLocation` (`self.WalkToPoint`) (`self.WalkToPosition`) false false))

(fn `Wait`
  (params (WaitTime :type "Float (double-precision)"))
  (`/Game/PointAndClick/Blueprints/BP_AdventureController.TaskWait` (`self.PlayerController`) WaitTime))