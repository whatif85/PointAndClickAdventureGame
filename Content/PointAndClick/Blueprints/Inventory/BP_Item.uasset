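; BP_Item is an inventory item for a point-and-click adventure, defining default responses to verb actions and item combining.
; Most verb events bark a stock refusal through ItemBark, which sends the text to AdventureController and interrupts the action; Walkto, Talkto and Give are empty.
; OnItemUsed compares the used item with InteractableItem, excluding the first enum value, then calls ItemCombineSuccess, which only prints, or ItemCombineFail, which barks.
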(event `/Game/PointAndClick/Blueprints/Interfaces/BPI_VerbInteraction.OnItemUsed`
  (params (Item :type "/Game/PointAndClick/Blueprints/Enums/ENUM_ItemList Enum" :default "NewEnumerator0"))
  (bind _interactableitem (`self.InteractableItem`))
  (if (and (`|EnumEquality` Item _interactableitem) (`|EnumInequality` _interactableitem "NewEnumerator0"))
    (`self.ItemCombineSuccess`)
    (else
      (`self.ItemCombineFail` "I can't use these things together."))))

(event `/Game/PointAndClick/Blueprints/Interfaces/BPI_VerbInteraction.OnWalkTo`)

(event `/Game/PointAndClick/Blueprints/Interfaces/BPI_VerbInteraction.OnPull`
  (`self.ItemBark` "That doesn't seem to move."))

(event `/Game/PointAndClick/Blueprints/Interfaces/BPI_VerbInteraction.OnPush`
  (`self.ItemBark` "That doesn't seem to move."))

(event `/Game/PointAndClick/Blueprints/Interfaces/BPI_VerbInteraction.OnUse`
  (`self.ItemBark` "That doesn't seem to work."))

(event `/Game/PointAndClick/Blueprints/Interfaces/BPI_VerbInteraction.OnTalkTo`)

(event `/Game/PointAndClick/Blueprints/Interfaces/BPI_VerbInteraction.OnLookAt`
  (`self.ItemBark` "I don't see anything special about it."))

(event `/Game/PointAndClick/Blueprints/Interfaces/BPI_VerbInteraction.OnClose`
  (`self.ItemBark` "That doesn't seem to close."))

(event `/Game/PointAndClick/Blueprints/Interfaces/BPI_VerbInteraction.OnOpen`
  (`self.ItemBark` "That doesn't seem to open."))

(event `/Game/PointAndClick/Blueprints/Interfaces/BPI_VerbInteraction.OnGive`)

(event `/Game/PointAndClick/Blueprints/Interfaces/BPI_VerbInteraction.OnPickUp`
  (`self.ItemBark` "I already have it."))

(fn `ItemCombineFail`
  (params (BarkText :type String))
  (`self.ItemBark` BarkText))

(fn `ItemCombineSuccess`
  (`KismetSystemLibrary.PrintString` null "Combine: SUCCESS"))