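; Orthographic follow camera for the point-and-click adventure that tracks the player within a bounded area.
; On BeginPlay it derives X/Y limits from the CameraConfines box, inset by half the ortho view size, then becomes the view target.
; Each tick it interpolates toward the player's capsule, clamps to those limits and moves the camera at fixed Z.
; The construction script sizes the confines box from ConfinesExtent.
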(event `self.ReceiveBeginPlay`
  (`self.GetCameraConfines`
    (:`Out`
      (`self.ActivateCamera`))))

(event `self.ReceiveTick`
  (params (DeltaSeconds :type "Float (single-precision)"))
  (set `self.DeltaSeconds` DeltaSeconds)
  (`/Engine/EditorBlueprintResources/StandardMacros.IsValid` (`self.Player`)
    (:`Is Valid`
      (`self.CamFollowPlayerX`
        (:`Out`
          (`self.CamFollowPlayerY`
            (:`Out`
              (`self.LerpWithinConfines`
                (:`Out`
                  (`self.SetCameraLocation`))))))))))

(fn `UserConstructionScript`
  (`BoxComponent.SetBoxExtent` (`self.CameraConfines`) (`self.ConfinesExtent`) true))